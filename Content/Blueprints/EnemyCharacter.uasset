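; Enemy character Blueprint that deals repeated contact damage to the hero and is destroyed when its own health runs out.
; AffectHealth passes the delta to CalculateHealth, then destroys the actor if IsDead is set.
; Overlapping a HeroCharacter starts a looping timer that applies Damage at AttacksPerSecond, cleared when that overlap ends.
; The construction script creates a dynamic material instance on the mesh to tint its body with EnemyColor.
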(event Custom|DamageTheHero
  (Default|AffectHealth (Variables|Default|GetHero) (Variables|Default|GetDamage)))

(event EventBeginPlay)

(event Collision|EventActorBeginOverlap
  (params (OtherActor :type Actor%20Object%20Reference))
  ;[1 1 1] Collision Test with Hero: Start
  (bind _ashero_character (Utilities|Casting|CastToHeroCharacter OtherActor))
  (Variables|Default|SetHero _ashero_character)
  ;[1 1 1] Timer: Damage per second
  (Utilities|Time|SetTimerbyFunctionName 0 "DamageTheHero" (/ 1.0 (Variables|Default|GetAttacksPerSecond)) true))

(event EventTick
  (params (DeltaSeconds :type Float%20%28single-precision%29)))

(event Collision|EventActorEndOverlap
  (params (OtherActor :type Actor%20Object%20Reference))
  ;[1 1 1] Collision Test with Hero: Stop
  (if (== OtherActor (Variables|Default|GetHero))
    (Utilities|Time|ClearTimerbyFunctionName 0 "DamageTheHero")))

(event EventAffectHealth
  (params (Delta :type Float%20%28single-precision%29))
  ;[1 1 1] Event: Affect Health
  (Class|BaseCharacter|CalculateHealth Delta)
  (if (Variables|Default|GetisDead)
    (Actor|DestroyActor)))

(fn ConstructionScript
  (bind _returnvalue (Rendering|Material|CreateDynamicMaterialInstance (Variables|Character|GetMesh) 0 0 :!class /Script/Engine.PrimitiveComponent))
  (bind _output_get (Variables|Default|SetDyna%20Mat _returnvalue))
  (Rendering|Material|SetVectorParameterValue (Variables|Default|GetDyna%20Mat) "BodyColor" (Variables|Default|GetEnemyColor) :!class /Script/Engine.MaterialInstanceDynamic))